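; Wind tail actor that drifts a Niagara effect through the wind field around the player.
; Periodically respawns above traced ground, or around the pawn if none is hit, randomizing oscillation type, phase and particle parameters.
; Samples WindManager every second as a force, integrating it on Tick to move the actor.
; Offsets the Niagara component by type (flat, vertical swing, spiral around the wind direction); destroys itself without a manager.
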(event `RetraceAtSpawn`
  (bind _returnvalue (`KismetMathLibrary.GetPI`))
  (bind _niagara (`self.Niagara`))
  (bind _lifetime (`self.LifeTime`))
  (bind _returnvalue_2 (`self.K2_GetActorLocation` (`Controller.K2_GetPawn` (`GameplayStatics.GetPlayerController` 0))))
  (`KismetSystemLibrary.K2_ClearAndInvalidateTimerHandle` (`self.TimerSpawn`))
  (`NiagaraComponent.ResetSystem` (`self.Niagara`))
  (set `self.Type` (select `int` (`KismetMathLibrary.RandomIntegerInRange` 0 2) :`0` "NewEnumerator0" :`1` "NewEnumerator1" :`2` "NewEnumerator2" :!type "/Game/WindSystem/E_WindTailType Enum")) ; Giv a new random oscillation type
  (bind (_outhit _returnvalue_3) (`KismetSystemLibrary.LineTraceSingle` :`Start` (+ _returnvalue_2 (0.0 0.0 5000.0)) :`End` (+ _returnvalue_2 (`KismetMathLibrary.MakeVector` (`KismetMathLibrary.RandomFloatInRange` -10000.0 10000.0) (`KismetMathLibrary.RandomFloatInRange` -10000.0 10000.0) -5000.0)) :`TraceChannel` "TraceTypeQuery1" :`DrawDebugType` "ForDuration")) ; Find a random location around the player
  (`self.K2_SetActorLocation` (`KismetMathLibrary.SelectVector` (+ (`.ImpactPoint` (`GameplayStatics.BreakHitResult` _outhit)) (`KismetMathLibrary.MakeVector` 0.0 0.0 (`KismetMathLibrary.RandomFloatInRange` 1000.0 3000.0))) (- _returnvalue_2 (`KismetMathLibrary.MakeVector` (`KismetMathLibrary.RandomFloatInRange` -4000.0 4000.0) (`KismetMathLibrary.RandomFloatInRange` -4000.0 4000.0) (`KismetMathLibrary.RandomFloatInRange` -2000.0 2000.0))) _returnvalue_3))
  (set `self.Velocity` (0.0 0.0 0.0))
  (set `self.LifeTime` (`KismetMathLibrary.RandomFloatInRange` 5.0 6.0))
  (set `self.Phase` (`KismetMathLibrary.RandomFloatInRange` _returnvalue (* _returnvalue -1.0))) ; restart the oscillation at a random phase
  (bind _output_get (set `self.NewTotalLifeTime` (`KismetMathLibrary.RandomFloatInRange` 10.0 30.0)))
  (`NiagaraComponent.SetVariableFloat` _niagara "user.DeathTime" _output_get)
  (`NiagaraComponent.SetVariableFloat` _niagara "user.width" (`KismetMathLibrary.RandomFloatInRange` 50.0 150.0))
  (`NiagaraComponent.SetVariableFloat` _niagara "user.Lifetime" _lifetime)
  (bind _returnvalue_4 (`KismetSystemLibrary.K2_SetTimerDelegate` (delegate `RetraceAtSpawn`) (+ (`self.NewTotalLifeTime`) 2.0 _lifetime))) ; Respawn the particle after the lifetime is passed
  (set `self.TimerSpawn` _returnvalue_4))

(event `Fetch force`
  (set `self.Force` (* (`/Game/WindSystem/BP_WindManager.Get wind direction at location` (`self.Wind manager`) (`self.K2_GetActorLocation`)) 10.0)))

(event `self.ReceiveBeginPlay`
  (`/Engine/EditorBlueprintResources/StandardMacros.IsValid` (`self.Wind manager`)
    (:`Is Valid`
      (`self.RetraceAtSpawn`)
      (`self.Fetch force`)
      (`self.SetActorTickEnabled` true)
      (`KismetSystemLibrary.K2_SetTimerDelegate` (delegate `Fetch force`) 1.0 true))
    (:`Is Not Valid`
      (`self.K2_DestroyActor`) ; If no manager, we can't sample the force\nso there is no point for this actor to\nexist
    )))

(event `self.ReceiveTick`
  (params (DeltaSeconds :type "Float (single-precision)"))
  (bind _returnvalue_location (`KismetMathLibrary.BreakTransform` (`self.GetTransform`)))
  (bind _returnvalue (`GameplayStatics.GetWorldDeltaSeconds`))
  (bind _returnvalue_location_2 (`KismetMathLibrary.BreakTransform` (`self.GetTransform`)))
  (bind _niagara (`self.Niagara`))
  (bind _returnvalue_2 (`KismetMathLibrary.Conv_VectorToRotator` (`self.Force`)))
  (bind _returnvalue_3 (+ (* (`self.TotalTime`) (`self.Frequency`)) (`self.Phase`)))
  (set `self.TotalTime` (+ DeltaSeconds (`self.TotalTime`))) ; total lifetime since the respawn
  ;[1 0.9198 0.3687] Force field base position update
  (set `self.Last Tick Position` (`self.K2_GetActorLocation`))
  (`self.K2_SetActorLocation` (+ (* (`self.Force`) _returnvalue _returnvalue 0.5) (* (`self.Velocity`) _returnvalue) (`self.Last Tick Position`)))
  (set `self.Velocity` (/ (- (`self.K2_GetActorLocation`) (`self.Last Tick Position`)) (`GameplayStatics.GetWorldDeltaSeconds`)))
  ;[1 0.5932 0.9335] Tail Rotation
  (switch `/Game/WindSystem/E_WindTailType` (`self.Type`)
    (:`NewEnumerator1`
      (`SceneComponent.K2_SetWorldLocation` _niagara (+ (`KismetMathLibrary.MakeVector` 0.0 0.0 (* (`KismetMathLibrary.Cos` (+ (* (`self.TotalTime`) (`self.Frequency`)) (`self.Phase`))) 1000.0)) _returnvalue_location) false false))
    (:`NewEnumerator2`
      (`SceneComponent.K2_SetWorldLocation` _niagara (+ (* (* (`KismetMathLibrary.Cos` _returnvalue_3) 1000.0) (`KismetMathLibrary.GetUpVector` _returnvalue_2)) (* (`KismetMathLibrary.GetRightVector` _returnvalue_2) (* (`KismetMathLibrary.Sin` _returnvalue_3) 1000.0)) _returnvalue_location_2) false false))))

(fn `PrintRotationArrows`
  (bind _returnvalue_location (`KismetMathLibrary.BreakTransform` (`self.GetTransform`)))
  (bind _returnvalue (`KismetMathLibrary.Conv_VectorToRotator` (`self.Force`)))
  (bind _returnvalue_2 (+ (* (`self.TotalTime`) (`self.Frequency`)) (`self.Phase`)))
  (`KismetSystemLibrary.DrawDebugArrow` _returnvalue_location (+ _returnvalue_location (* (* (`KismetMathLibrary.Cos` _returnvalue_2) 1000.0) (`KismetMathLibrary.GetUpVector` _returnvalue))) 100.0 (struct :`G` 0.699428 :`B` 1.0 :`A` 1.0) 0.0 50.0)
  (`KismetSystemLibrary.DrawDebugArrow` _returnvalue_location (+ (* (`KismetMathLibrary.GetRightVector` _returnvalue) (* (`KismetMathLibrary.Sin` _returnvalue_2) 1000.0)) _returnvalue_location) 100.0 (struct :`R` 1.0 :`G` 0.036458 :`B` 0.036458 :`A` 1.0) 0.0 50.0)
  (return))

(fn `UserConstructionScript`)