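; Wind manager that bakes a world wind field from Source, Well and Booster actors into render targets and spawns BP_WindTail trails.
; Each redraw sums radial pushes, pulls and distance-attenuated directional boosts per texel, at terrain heights line-traced once and cached, encoding the force as color.
; A looping timer alternates redraws between two buffers, while Tick eases the MP_Wind "Alpha" parameter along a tanh curve to crossfade them.
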(event `self.ReceiveBeginPlay`
  (`self.CleanExtremaList`)
  (bind _returnvalue (`KismetMaterialLibrary.GetScalarParameterValue` "/Game/WindSystem/MP_Wind.MP_Wind" "World Size"))
  (set `self.Size` _returnvalue)
  (set `self.Start Call` true)
  (`KismetSystemLibrary.K2_SetTimer` null "CacheNewWind" 15.0 true)
  (`KismetSystemLibrary.Delay` 1.0)
  (`self.CacheNewWind`)
  (`KismetSystemLibrary.Delay` 1.0)
  (for _ (range 1 (+ (`self.Trails`) 1))
    (`|SpawnActorFromClass` "/Game/WindSystem/BP_WindTail.BP_WindTail_C" (`KismetMathLibrary.MakeTransform` (0.0 0.0 0.0)) "Undefined" "MultiplyWithRoot" null self null)))

(event `RedrawAndReshape`
  (`self.Redraw` "/Game/WindSystem/RT_WindBufferA.RT_WindBufferA") ; called in at max 2 s
  (`KismetMaterialLibrary.SetScalarParameterValue` "/Game/WindSystem/MP_Wind.MP_Wind" "Alpha"))

(event `self.ReceiveTick`
  (params (DeltaSeconds :type "Float (single-precision)"))
  (bind _returnvalue (/ (+ (`/Game/WindSystem/BPFL_Lerp.Tanh` (`self.CurrenTime`) 6.0 0.5) 1.0) 2.0))
  (if (< (`KismetMathLibrary.Abs` (- (`self.TargetAlpha`) (`self.CurrentAlpha`))) 0.001)
    (set `self.CurrenTime` 0.0)
    (else
      (set `self.CurrenTime` (+ (`self.CurrenTime`) (* (/ DeltaSeconds 10.0) (`self.Interpolation Exponenent`))))
      (set `self.CurrentAlpha` (`KismetMathLibrary.SelectFloat` (- 1.0 _returnvalue) _returnvalue (== (`self.TargetAlpha`) 0.0))) ; smoth evolution of\nthe interpolation factor
      (`KismetMaterialLibrary.SetScalarParameterValue` "/Game/WindSystem/MP_Wind.MP_Wind" "Alpha" (`self.CurrentAlpha`)))))

(fn `BoosterPotential`
  (params (Location :type "Vector Structure") (`Source Location` :type "Vector Structure") (Force :type "Float (double-precision)") (Orientation :type "Vector Structure") (Power :type "Float (double-precision)"))
  (returns (ReturnValue :type "Vector Structure"))
  (return (* 10000.0 Force (/ Orientation (`KismetMathLibrary.MultiplyMultiply_FloatFloat` (`KismetMathLibrary.VSize` (- Location `Source Location`)) Power)))))

(fn `CacheNewWind`
  (if (`self.Start Call`)
    (set `self.Start Call` false)
    (`self.Redraw` "/Game/WindSystem/RT_WindBufferA.RT_WindBufferA")
    (set `self.TargetAlpha` 0.0)
    (set `self.CurrentAlpha` 0.0)
    (set `self.WindCachedInBufferA` true)
    (`KismetMaterialLibrary.SetScalarParameterValue` "/Game/WindSystem/MP_Wind.MP_Wind" "Alpha")
    (elif (`self.WindCachedInBufferA`)
      (`self.Redraw` "/Game/WindSystem/RT_WindBufferB.RT_WindBufferB")
      (set `self.TargetAlpha` 1.0)
      (set `self.WindCachedInBufferA` false)
      (else
        (`self.Redraw` "/Game/WindSystem/RT_WindBufferA.RT_WindBufferA")
        (set `self.TargetAlpha` 0.0)
        (set `self.WindCachedInBufferA` true)))))

(fn `CleanExtremaList`
  (locals (Removed :type Integer))
  (for _index (range (+ (`KismetArrayLibrary.Array_LastIndex` (`self.Extremas`)) 1))
    (bind _returnvalue (- _index (`local.Removed`)))
    (`/Engine/EditorBlueprintResources/StandardMacros.IsValid` (`|GetArrayItem` (`self.Extremas`) _returnvalue)
      (:`Is Not Valid`
        (`KismetArrayLibrary.Array_Remove` (`self.Extremas`) _returnvalue)
        (`/Engine/EditorBlueprintResources/StandardMacros.IncrementInt` (`local.Removed`))))))

(fn `ComputeHight`
  (params (`Text Size` :type "Vector2D Structure"))
  (bind (_x _y) (`KismetMathLibrary.BreakVector2D` `Text Size`))
  (bind (_x_2 _y_2) (`KismetMathLibrary.BreakVector2D` `Text Size`))
  (bind _returnvalue (`KismetMathLibrary.FTrunc` _y))
  (bind _returnvalue_2 (`KismetMathLibrary.FTrunc` _x))
  (bind _returnvalue_3 (/ (`self.Size`) 2.0))
  (`KismetArrayLibrary.Array_Resize` (`self.LandscapePositions`) (* _returnvalue_2 _returnvalue)) ; preallocation
  (for _index (range (+ _returnvalue_2 1))
    (for _index_2 (range (+ _returnvalue 1))
      (bind _returnvalue_4 (`KismetMathLibrary.MakeVector` (- (* _index (/ (`self.Size`) _x_2)) _returnvalue_3) (- (* _index_2 (/ (`self.Size`) _y_2)) _returnvalue_3) -1.0))
      (bind _outhit (`KismetSystemLibrary.LineTraceSingle` :`Start` (+ _returnvalue_4 (0.0 0.0 12000.0)) :`End` _returnvalue_4 :`TraceChannel` "TraceTypeQuery1" :`DrawTime` 1.5))
      (`KismetArrayLibrary.Array_Set` (`self.LandscapePositions`) (* (- _index 1) _index_2) (.z (`.Location` (`GameplayStatics.BreakHitResult` _outhit)))))))

(fn `Get wind direction at location`
  (params (location :type "Vector Structure"))
  (returns (Force :type "Vector Structure"))
  (locals (`Total Force` :type "Vector Structure"))
  (for _array_element (`self.Extremas`)
    (bind _type (`/Game/WindSystem/BP_MasterWindExtremum.Type` _array_element))
    (switch `/Game/WindSystem/E_WindExtremumType` _type
      (:`NewEnumerator0`
        (bind _returnvalue_location (`KismetMathLibrary.BreakTransform` (`self.GetTransform` _array_element)))
        (bind _influence (`/Game/WindSystem/BP_MasterWindExtremum.Influence` _array_element))
        (set `local.Total Force` (+ (`self.SinglePotential` (`local.location`) _returnvalue_location (* _influence (select `/Game/WindSystem/E_WindExtremumType` _type :`NewEnumerator0` 1.0 :`NewEnumerator1` -1.0))) (`local.Total Force`)) :!label _label))
      (:`NewEnumerator1`
        (goto _label))
      (:`NewEnumerator2`
        (bind _returnvalue_location_2 (`KismetMathLibrary.BreakTransform` (`self.GetTransform` _array_element)))
        (set `local.Total Force` (+ (`self.BoosterPotential` (`local.location`) _returnvalue_location_2 _influence (`SceneComponent.GetForwardVector` (`/Game/WindSystem/BP_MasterWindExtremum.Arrow` _array_element)) (`/Game/WindSystem/BP_MasterWindExtremum.Power` _array_element)) (`local.Total Force`))))))
  (return (`local.Total Force`)))

(fn `Redraw`
  (params (TextureRenderTarget :type "TextureRenderTarget2D Object Reference"))
  (bind _returnvalue (/ (`self.Size`) 2.0))
  (bind (_canvas _size _context) (`KismetRenderingLibrary.BeginDrawCanvasToRenderTarget` TextureRenderTarget))
  (`|ExecutionSequence`
    (:`then_0`
      (if (`KismetArrayLibrary.Array_IsEmpty` (`self.LandscapePositions`))
        (`self.ComputeHight` _size)))
    (:`then_1`
      (bind (_x _y) (`KismetMathLibrary.BreakVector2D` _size))
      (for _index (range (+ (`KismetMathLibrary.FTrunc` _x) 1))
        (for _index_2 (range (+ (`KismetMathLibrary.FTrunc` _y) 1))
          (bind (_x_2 _y_2) (`KismetMathLibrary.BreakVector2D` _size))
          (`Canvas.K2_DrawTexture` _canvas null (`KismetMathLibrary.MakeVector2D` (`KismetMathLibrary.Conv_IntToDouble` _index_2) (`KismetMathLibrary.Conv_IntToDouble` _index)) (1.0 1.0) (0.0 0.0) (1.0 1.0) (`KismetMathLibrary.Conv_VectorToLinearColor` (/ (+ (/ (`self.Get wind direction at location` (`KismetMathLibrary.MakeVector` (- (* _index (/ (`self.Size`) _x_2)) _returnvalue) (- (* _index_2 (/ (`self.Size`) _y_2)) _returnvalue) (`|GetArrayItem` (`self.LandscapePositions`) (* (- _index 1) _index_2)))) 100.0) (1.0 1.0 1.0)) (2.0 2.0 2.0))) "BLEND_Opaque" 0.0 (0.5 0.5))))
      (`KismetRenderingLibrary.EndDrawCanvasToRenderTarget` _context)
      (if (`self.AskReshape`)
        (`/Game/WindSystem/BP_WindSampler.Redraw` (`self.Sampler`))
        (set `self.AskReshape` false)))))

(fn `SinglePotential`
  (params (Location :type "Vector Structure") (`Source Location` :type "Vector Structure") (Force :type "Float (double-precision)"))
  (returns (ReturnValue :type "Vector Structure"))
  (bind _returnvalue (- Location `Source Location`))
  (return (* (/ _returnvalue (`KismetMathLibrary.VSize` _returnvalue)) (`local.Force`))))

(fn `UserConstructionScript`
  (locals (NewLocalVar :type Boolean))
  (for _array_element (`self.Extremas`)
    (set `/Game/WindSystem/BP_MasterWindExtremum.Manager` self _array_element)))