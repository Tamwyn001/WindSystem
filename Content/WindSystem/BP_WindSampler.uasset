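; BP_WindSampler is a debug-style visualizer that shows the wind field as a 3D grid of arrows.
; Redraw rebuilds an instanced static mesh, querying WindManager at each grid point around the actor and rotating each arrow along the wind direction.
; Per-instance custom data colors arrows from green to red by force magnitude.
; BeginPlay and the construction script do nothing; their Redraw and sampler-registration nodes are disconnected.
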(event `self.ReceiveBeginPlay`)

(fn `Redraw`
  (locals (X :type Integer) (Y :type Integer) (Z :type Integer) (Force :type "Vector Structure") (Color :type "Vector Structure"))
  (bind _distance (`self.Distance`))
  (bind _returnvalue (* (`KismetMathLibrary.MakeVector` (`KismetMathLibrary.Conv_IntToDouble` (`local.X`)) (`KismetMathLibrary.Conv_IntToDouble` (`local.Y`)) (`KismetMathLibrary.Conv_IntToDouble` (`local.Z`))) _distance))
  (if (`KismetSystemLibrary.IsValid` (`self.Arrows`))
    (`ActorComponent.K2_DestroyComponent` (`self.Arrows`)))
  (bind _returnvalue_2 (`AddComponent|NODE_AddInstancedStaticMeshComponent-2`))
  (set `self.Arrows` _returnvalue_2)
  (for _index (range (+ (`KismetMathLibrary.FTrunc` (.x (`self.SystemSize`))) 1))
    (set `local.X` _index)
    (for _index_2 (range (+ (`KismetMathLibrary.FTrunc` (.y (`self.SystemSize`))) 1))
      (set `local.Y` _index_2)
      (for _index_3 (range (+ (`KismetMathLibrary.FTrunc` (.z (`self.SystemSize`))) 1))
        (set `local.Z` _index_3)
        (set `local.Force` (`/Game/WindSystem/BP_Windmanager.Get wind direction at location` (`self.WindManager`) (+ _returnvalue (`self.K2_GetActorLocation`))))
        (bind _returnvalue_3 (`InstancedStaticMeshComponent.AddInstance` (`self.Arrows`) (`KismetMathLibrary.MakeTransform` _returnvalue (`KismetMathLibrary.Conv_VectorToRotator` (`local.Force`)) (* (`KismetMathLibrary.Conv_DoubleToVector` (/ _distance 200.0)) (1.75 2.0 2.0))) false))
        (bind _output_get (set `local.Color` (`KismetMathLibrary.VLerp` (`KismetMathLibrary.Conv_LinearColorToVector` (`KismetMathLibrary.LinearColor_Green`)) (`KismetMathLibrary.Conv_LinearColorToVector` (`KismetMathLibrary.LinearColor_Red`)) (/ (`KismetMathLibrary.VSize` (`local.Force`)) (`self.ColorerForceUpperBound`)))))
        (`InstancedStaticMeshComponent.SetCustomDataValue` (`self.Arrows`) _returnvalue_3 0 (.x _output_get) false)
        (`InstancedStaticMeshComponent.SetCustomDataValue` (`self.Arrows`) _returnvalue_3 1 (.y _output_get) false)
        (`InstancedStaticMeshComponent.SetCustomDataValue` (`self.Arrows`) _returnvalue_3 2 (.z _output_get) false)))))

(fn `UserConstructionScript`)