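; BP_MasterWindExtremum is a wind system point actor, typed as Source, Well or Booster, with Influence and Power controlling its force falloff.
; Construction sets the type's sprite, shows an arrow only for Boosters, locks Power to 1 otherwise, then draws labeled 75/50/25% debug rings.
; RedrawForceFalloff also refreshes BP_WindManager, except when called from construction.
; An optional Tick mode orbits the actor around a point offset from its start location.
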(event `self.ReceiveBeginPlay`
  (set `self.Center` (+ (`self.K2_GetActorLocation`) (3000.0 3000.0 0.0))))

(event `self.ReceiveTick`
  (params (DeltaSeconds :type "Float (single-precision)"))
  (bind _t (`self.T`))
  (if (`self.Rotate Arround center`)
    (`self.K2_SetActorLocation` (+ (`self.Center`) (* (`KismetMathLibrary.MakeVector` (`KismetMathLibrary.Cos` (+ 0.0 (* _t 0.3))) (`KismetMathLibrary.Sin` (+ 0.0 (* _t 0.3)))) (`KismetMathLibrary.VSize` (- (`self.K2_GetActorLocation`) (`self.Center`))))))
    (set `self.T` (+ (`self.T`) DeltaSeconds))))

(fn `RedrawForceFalloff`
  (locals (Rad1 :type "Float (double-precision)" :default 0.0) (Rad2 :type "Float (double-precision)" :default 0.0) (Rad3 :type "Float (double-precision)"))
  (bind _returnvalue_location (`KismetMathLibrary.BreakTransform` (`self.GetTransform`)))
  (bind _returnvalue_location_2 (`KismetMathLibrary.BreakTransform` (`self.GetTransform`)))
  (bind _returnvalue_location_3 (`KismetMathLibrary.BreakTransform` (`self.GetTransform`)))
  (if (`self.ConstructionJustExecuted`)
    (set `self.ConstructionJustExecuted` false)
    (else
      (bind _returnvalue (`GameplayStatics.GetActorOfClass` "/Game/WindSystem/BP_Windmanager.BP_WindManager_C"))
      (`/Game/WindSystem/BP_Windmanager.RedrawAndReshape` _returnvalue)))
  (bind _output_get (set `local.Rad2` (`KismetMathLibrary.MultiplyMultiply_FloatFloat` (/ (* (`self.Influence`) 100.0) 0.5) (/ 1.0 (`self.Power`)))))
  (`KismetSystemLibrary.DrawDebugCircle` (`self.K2_GetActorLocation`) _output_get 12 (struct :`R` 1.0 :`G` 0.494728 :`B` 0.081323 :`A` 1.0) 3.0 (`KismetMathLibrary.FClamp` (`KismetMathLibrary.MultiplyMultiply_FloatFloat` (/ (`local.Rad2`) 2000.0) 2.0) 100.0 2700.0) (1.0 0.0 0.0) (0.0 1.0 0.0))
  (bind _output_get_2 (set `local.Rad3` (`KismetMathLibrary.MultiplyMultiply_FloatFloat` (/ (* (`self.Influence`) 100.0) 0.25) (/ 1.0 (`self.Power`)))))
  (`KismetSystemLibrary.DrawDebugCircle` (`self.K2_GetActorLocation`) _output_get_2 12 (struct :`R` 0.628041 :`G` 1.0 :`B` 0.056731 :`A` 1.0) 3.0 (`KismetMathLibrary.FClamp` (`KismetMathLibrary.MultiplyMultiply_FloatFloat` (/ (`local.Rad3`) 2000.0) 2.0) 100.0 2700.0) (1.0 0.0 0.0) (0.0 1.0 0.0))
  (bind _output_get_3 (set `local.Rad1` (`KismetMathLibrary.MultiplyMultiply_FloatFloat` (/ (* (`self.Influence`) 100.0) 0.75) (/ 1.0 (`self.Power`)))))
  (`KismetSystemLibrary.DrawDebugCircle` (`self.K2_GetActorLocation`) _output_get_3 12 (struct :`R` 1.0 :`G` 0.036458 :`B` 0.036458 :`A` 1.0) 3.0 (`KismetMathLibrary.FClamp` (`KismetMathLibrary.MultiplyMultiply_FloatFloat` (/ (`local.Rad1`) 2000.0) 2.0) 100.0 2700.0) (1.0 0.0 0.0) (0.0 1.0 0.0))
  (`KismetSystemLibrary.DrawDebugString` (+ (* (/ (`local.Rad1`) 2.0) (1.0 0.0 0.0)) _returnvalue_location_2) "75%" null (struct :`R` 1.0 :`G` 0.036458 :`B` 0.036458 :`A` 1.0) 3.0)
  (`KismetSystemLibrary.DrawDebugString` (+ (* (/ (+ (`local.Rad1`) (`local.Rad2`)) 2.0) (1.0 0.0 0.0)) _returnvalue_location_3) "50%" null (struct :`R` 1.0 :`G` 0.494728 :`B` 0.081323 :`A` 1.0) 3.0)
  (`KismetSystemLibrary.DrawDebugString` (+ (* (/ (+ (`local.Rad3`) (`local.Rad2`)) 2.0) (1.0 0.0 0.0)) _returnvalue_location) "25%" null (struct :`R` 0.628041 :`G` 1.0 :`B` 0.056731 :`A` 1.0) 3.0))

(fn `UserConstructionScript`
  (`|ExecutionSequence`
    (:`then_0`
      (if (not (`|EnumEquality` (`self.Type`) "NewEnumerator2"))
        (set `self.Power` 1.0)))
    (:`then_1`
      (`BillboardComponent.SetSprite` (`self.Billboard`) (select `/Game/WindSystem/E_WindExtremumType` (`self.Type`) :`NewEnumerator0` "/Engine/EditorMaterials/Anchor.Anchor" :`NewEnumerator1` "/Engine/MobileResources/HUD/AnalogHat.AnalogHat" :`NewEnumerator2` "/Engine/EngineResources/AICON-Red.AICON-Red" :!type "Texture2D Object Reference"))
      (`SceneComponent.SetVisibility` (`self.Arrow`) (`|EnumEquality` (`self.Type`) "NewEnumerator2") false)
      (set `ArrowComponent.ArrowSize` (* (`self.Influence`) 6.0) (`self.Arrow`))
      (set `self.ConstructionJustExecuted` true)
      (`self.RedrawForceFalloff`))))